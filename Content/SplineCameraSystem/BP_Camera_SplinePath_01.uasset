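; Spline camera path actor that takes over the player's view when the pawn overlaps trigger boxes at either end of its ground spline.
; Each tick, the camera follows the camera spline by elapsed time, nearest spline point, or player progress along sampled ground points scaled by length ratio.
; Per-point data sets offset, rotation and FOV, optionally aiming at the player instead.
; Activation deactivates other paths; timed cutscene runs can restore the previous camera or path.
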(event `self.ReceiveBeginPlay`
  (bind _camerapathactors (`self.CameraPathActors`))
  ;[1 1 1] Event: Begin Play
  ;[1 1 1] Store all camera paths so we can deactivate them when they become inactive without having to make expensive GetAllActors calls
  (`KismetArrayLibrary.Array_Clear` _camerapathactors)
  (`KismetArrayLibrary.Array_Resize` _camerapathactors)
  (bind _outactors (`GameplayStatics.GetAllActorsOfClass` "BP_Camera_SplinePath_01_C"))
  (for _array_element _outactors
    (bind _asbp_camera_spline_path_01 (cast `/Game/SplineCameraSystem/BP_Camera_SplinePath_01` _array_element))
    (`KismetArrayLibrary.Array_Add` (`self.CameraPathActors`) _asbp_camera_spline_path_01)))

(event `self.PathStartTrigger.OnComponentBeginOverlap`
  (params (OverlappedComponent :type "PrimitiveComponent Object Reference") (OtherActor :type "Actor Object Reference") (OtherComp :type "PrimitiveComponent Object Reference") (OtherBodyIndex :type Integer) (bFromSweep :type Boolean) (SweepResult :type "HitResult Structure (by ref)"))
  ;[1 1 1] Box Component Overlaps: Switch active camera when trigger areas are crossed
  (if (== OtherActor (`GameplayStatics.GetPlayerPawn` 0))
    (`self.Activate` :!label _label)))

(event `self.PathEndTrigger.OnComponentBeginOverlap`
  (params (OverlappedComponent :type "PrimitiveComponent Object Reference") (OtherActor :type "Actor Object Reference") (OtherComp :type "PrimitiveComponent Object Reference") (OtherBodyIndex :type Integer) (bFromSweep :type Boolean) (SweepResult :type "HitResult Structure (by ref)"))
  ;[1 1 1] Box Component Overlaps: Switch active camera when trigger areas are crossed
  (if (== (`GameplayStatics.GetPlayerPawn` 0) OtherActor)
    (goto _label)))

(event `self.ReceiveTick`
  (params (DeltaSeconds :type "Float (single-precision)"))
  (bind _grounddatapoints (`self.GroundDataPoints`))
  (bind _camerapath (`self.CameraPath`))
  (bind _camera (`self.Camera`))
  (bind _camera_2 (`self.Camera`))
  (bind _currenttime (`self.CurrentTime`))
  (bind _cameratrackduration (`self.CameraTrackDuration`))
  (bind _returnvalue (* (`self.GroundPathDistance`) (`self.CameraToPathRatio`)))
  (bind (_output_fov _output_offset) (break `/Game/SplineCameraSystem/Struct_CameraTrackData` (`|GetArrayItem` (`self.CameraDataPoints`) (`self.ClosestPointIndex`))))
  (bind (_output_fov_2 _output_offset_2 _output_rotation) (break `/Game/SplineCameraSystem/Struct_CameraTrackData` (`|GetArrayItem` (`self.CameraDataPoints`) (`self.ClosestPointToCameraIndex`))))
  (bind _output_fov_3 (break `/Game/SplineCameraSystem/Struct_CameraTrackData` (`|GetArrayItem` (`self.CameraDataPoints`) (`self.ClosestPointToCameraIndex`))))
  (bind (_output_location _output_rotation_2 _output_distancealongspline) (break `/Game/SplineCameraSystem/Struct_SplineLocation` (`|GetArrayItem` _grounddatapoints (`self.ClosestPointIndex`))))
  (bind (_output_location_2 _output_rotation_3 _output_distancealongspline_2) (break `/Game/SplineCameraSystem/Struct_SplineLocation` (`|GetArrayItem` _grounddatapoints (`self.SecondClosestPointIndex`))))
  (bind (_output_location_3 _output_rotation_4 _output_distancealongspline_3) (break `/Game/SplineCameraSystem/Struct_SplineLocation` (`|GetArrayItem` (`self.GroundDataPoints`) (`self.ClosestPointIndex`))))
  (bind (_output_location_4 _output_rotation_5 _output_distancealongspline_4) (break `/Game/SplineCameraSystem/Struct_SplineLocation` (`|GetArrayItem` (`self.GroundDataPoints`) (`self.SecondClosestPointIndex`))))
  (set `self.DeltaTime` DeltaSeconds)
  ;[1 1 1] Event Tick: Stash the time since last tick for easy use later, if this path is active we're gonna do alot
  (if (> (`self.TimeSinceActivation`) (`self.CameraTransitionToNewCameraSpeed`))
    (if (`self.Active`)
      (set `self.CurrentTime` (+ (`self.CurrentTime`) (`self.DeltaTime`)))
      (if (`self.UseCameraPathOnly`)
        ;[1 1 1] Find the closest spline point along the camera path to the player (for when bcamerapathonly is set)
        (set `self.ClosestPointIndex` -1)
        (set `self.ClosestPointDistance` 9999999999.0)
        (for _index (range (`SplineComponent.GetNumberOfSplinePoints` (`self.CameraPath`)))
          (set `self.CurrentPointDistance` (`KismetMathLibrary.VSize` (- (`SplineComponent.GetWorldLocationAtSplinePoint` (`self.CameraPath`) _index) (`self.K2_GetActorLocation` (`GameplayStatics.GetPlayerPawn` 0)))))
          (if (< (`self.CurrentPointDistance`) (`self.ClosestPointDistance`))
            (set `self.ClosestPointIndex` _index)
            (set `self.ClosestPointDistance` (`self.CurrentPointDistance`))))
        (else
          ;[1 1 1] Find the closest spline point along the ground path to the player (for when bcamerapathonly is not set)
          (set `self.ClosestPointIndex` 0)
          (set `self.ClosestPointDistance` 9999999999.0)
          (for _index_2 (range (`KismetArrayLibrary.Array_Length` (`self.GroundDataPoints`)))
            (bind _output_location_5 (break `/Game/SplineCameraSystem/Struct_SplineLocation` (`|GetArrayItem` (`self.GroundDataPoints`) _index_2)))
            (set `self.CurrentPointDistance` (`KismetMathLibrary.VSize` (- _output_location_5 (`self.K2_GetActorLocation` (`GameplayStatics.GetPlayerPawn` 0)))))
            (if (< (`self.CurrentPointDistance`) (`self.ClosestPointDistance`))
              (set `self.ClosestPointIndex` _index_2)
              (set `self.ClosestPointDistance` (`self.CurrentPointDistance`))))
          ;[1 1 1] Find the second closest spline point along the ground path to the player (for when bcamerapathonly is not set)
          (set `self.SecondClosestPointIndex` 0)
          (set `self.SecondClosestPointDistance` 99999999999.0)
          (for _index_3 (range (`KismetArrayLibrary.Array_Length` (`self.GroundDataPoints`)))
            (if (!= _index_3 (`self.ClosestPointIndex`))
              (bind _output_location_6 (break `/Game/SplineCameraSystem/Struct_SplineLocation` (`|GetArrayItem` (`self.GroundDataPoints`) _index_3)))
              (set `self.CurrentPointDistance` (`KismetMathLibrary.VSize` (- _output_location_6 (`self.K2_GetActorLocation` (`GameplayStatics.GetPlayerPawn` 0)))))
              (if (< (`self.CurrentPointDistance`) (`self.SecondClosestPointDistance`))
                (set `self.SecondClosestPointIndex` _index_3)
                (set `self.SecondClosestPointDistance` (`self.CurrentPointDistance`)))))
          ;[1 1 1] If the distance to the second closest point from the first is greater than the distance from closest to second closest then the player is beyond the start or end point so just use those as the closest and second closest to avoid jitters
          (if (< (`KismetMathLibrary.Abs` (- _output_distancealongspline _output_distancealongspline_2)) (`self.SecondClosestPointDistance`))
            (set `self.SecondClosestPointIndex` (`self.ClosestPointIndex`))
            (set `self.SecondClosestPointDistance` (`self.ClosestPointDistance`)))
          ;[1 1 1] Split the distance between the closest and second closest points to the player to figure out where along the spline the player is "really" closest to.
          (bind _output_get (set `self.GroundPathDistance` (`KismetMathLibrary.Lerp` _output_distancealongspline_3 _output_distancealongspline_4 (/ (`self.ClosestPointDistance`) (`self.SecondClosestPointDistance`)))))
          (if (`self.ShowGroundPathDensityArrows`)
            (`SceneComponent.K2_SetWorldLocation` (`self.PlayerPositionIndicator`) (`SplineComponent.GetWorldLocationAtDistanceAlongSpline` (`self.GroundPath`) _output_get) false false))))
      ;[1 1 1] Find the closest spline point along the camera path to the player (for when bcamerapathonly is set)
      (set `self.ClosestPointToCameraIndex` 0)
      (set `self.ClosestPointToCameraDistance` 9999999999.0)
      (for _index_4 (range (`SplineComponent.GetNumberOfSplinePoints` (`self.CameraPath`)))
        (set `self.CurrentPointDistance` (`KismetMathLibrary.VSize` (- (`SplineComponent.GetWorldLocationAtSplinePoint` (`self.CameraPath`) _index_4) (`SceneComponent.K2_GetComponentLocation` (`self.Camera`)))))
        (if (< (`self.CurrentPointDistance`) (`self.ClosestPointToCameraDistance`))
          (set `self.ClosestPointToCameraIndex` _index_4)
          (set `self.ClosestPointToCameraDistance` (`self.CurrentPointDistance`))))
      ;[1 1 1] Move camera along spline based on either A: Time Tracking (good for videos) B: Player distance along lower spline
      (`SceneComponent.K2_SetWorldLocation` (`self.Camera`) (`KismetMathLibrary.SelectVector` (+ (`SplineComponent.GetWorldLocationAtTime` (`self.CameraPath`) (`KismetMathLibrary.SelectFloat` _currenttime _cameratrackduration (<= _currenttime _cameratrackduration)) false) _output_offset) (`KismetMathLibrary.VInterpTo` (`SceneComponent.K2_GetComponentLocation` (`self.Camera`)) (+ _output_offset (`KismetMathLibrary.SelectVector` (`SplineComponent.GetWorldLocationAtSplinePoint` _camerapath (`self.ClosestPointIndex`)) (`SplineComponent.GetWorldLocationAtDistanceAlongSpline` _camerapath _returnvalue) (`self.UseCameraPathOnly`))) (`GameplayStatics.GetWorldDeltaSeconds`) (`self.CameraMovementSpeed`)) (`self.CameraMoveOverTime`)) false false)
      ;[1 1 1] Rotate camera base on either A: Facing directly at player B: Camera path spline rotation at camera location
      (`SceneComponent.K2_SetWorldRotation` _camera (`|EaseFunction` "Linear" (* (`self.DeltaTime`) (`self.CameraRotationSpeed`)) (`SceneComponent.K2_GetComponentRotation` _camera) (`KismetMathLibrary.SelectRotator` (`KismetMathLibrary.ComposeRotators` (`SplineComponent.GetWorldRotationAtDistanceAlongSpline` (`self.CameraPath`) _returnvalue) _output_rotation) (`KismetMathLibrary.FindLookAtRotation` (`SceneComponent.K2_GetComponentLocation` (`self.Camera`)) (`self.K2_GetActorLocation` (`GameplayStatics.GetPlayerPawn` 0))) (`self.CameraUseTrackDataPointRotation`))) false false)
      ;[1 1 1] Adjust FoV based on closest camera track data point
      (set `CameraComponent.FieldOfView` (`KismetMathLibrary.FInterpTo` (`CameraComponent.FieldOfView` _camera_2) (`KismetMathLibrary.SelectFloat` _output_fov_3 90.0 (> _output_fov_3 30.0)) (`self.DeltaTime`) (`self.CameraFOVChangeSpeed`)) _camera_2)
      ;[1 1 1] Deactivate this camera if this cutscene run has completed
      (if (and (`self.CameraMoveOverTime`) (>= (`self.ReturnToLastCameraDelay`) 0.0) (>= (`self.CurrentTime`) (+ (`self.CameraTrackDuration`) (`self.ReturnToLastCameraDelay`))))
        (`self.Deactivate`)))
    (else
      (set `self.TimeSinceActivation` (+ (`self.TimeSinceActivation`) (`self.DeltaTime`))))))

(fn `Activate`
  (if (not (`self.Disabled`))
    ;[1 1 1] If this is a move over time path (cutscene style) store the last camera that was active so we can reset to it later
    (if (`self.CameraMoveOverTime`)
      (bind _ascamera_actor (cast `CameraActor` (`Controller.GetViewTarget` (`GameplayStatics.GetPlayerController` 0))))
      (set `self.OldCamera` _ascamera_actor))
    ;[1 1 1] Deactivate any other camera paths in the level before making this one active and store the last active one for easy access later
    (for _array_element (`self.CameraPathActors`)
      (if (!= _array_element self)
        (if (`/Game/SplineCameraSystem/BP_Camera_SplinePath_01.Active` _array_element)
          (`self.Deactivate` _array_element)
          (set `self.OldCameraPath` _array_element))))
    (set `self.Active` true)
    (`SceneComponent.K2_SetWorldLocation` (`self.Camera`) (`SceneComponent.K2_GetComponentLocation` (`self.Camera`)) false false)
    (`PlayerController.SetViewTargetWithBlend` (`GameplayStatics.GetPlayerController` 0) self (`self.CameraTransitionToNewCameraSpeed`) "VTBlend_Cubic" 0.0 false)
    (set `self.TimeSinceActivation` -0.01)))

(fn `Deactivate`
  (bind _oldcamera (`self.OldCamera`))
  (bind _oldcamerapath (`self.OldCameraPath`))
  (set `self.Active` false)
  ;[1 1 1] If a different camera was active before this cutscene style camera ran then restore it
  (if (and (!= _oldcamera null) (`self.CameraMoveOverTime`) (== (`self.OldCameraPath`) null))
    (`PlayerController.SetViewTargetWithBlend` (`GameplayStatics.GetPlayerController` 0) _oldcamera (`self.CameraTransitionToNewCameraSpeed`) "VTBlend_Cubic" 0.0 false)
    (set `self.OldCamera` null)
    (if (`self.ResetAfterComplete`) :!label _label
      (set `self.Disabled` false)
      (`self.Reset`)
      (else
        (set `self.Disabled` true)))
    (else
      ;[1 1 1] If we had a previous camera path before this cutscene then reactivate it
      (if (and (!= _oldcamerapath null) (`self.CameraMoveOverTime`))
        (`self.Activate` _oldcamerapath)
        (set `self.OldCameraPath` null)
        (goto _label)))))

(fn `Reset`
  (bind _camera (`self.Camera`))
  (bind _camerapath (`self.CameraPath`))
  (bind (_output_fov _output_offset _output_rotation) (break `/Game/SplineCameraSystem/Struct_CameraTrackData` (`|GetArrayItem` (`self.CameraDataPoints`))))
  (set `self.Active` false)
  (set `self.CurrentTime` 0.0)
  (`SceneComponent.K2_SetWorldTransform` _camera (`KismetMathLibrary.MakeTransform` (+ (`SplineComponent.GetWorldLocationAtSplinePoint` _camerapath 0) _output_offset) (`KismetMathLibrary.ComposeRotators` (`SplineComponent.GetWorldRotationAtDistanceAlongSpline` _camerapath 0.0) _output_rotation)) false false)
  (set `CameraComponent.FieldOfView` (`KismetMathLibrary.SelectFloat` _output_fov 90.0 (> _output_fov 0.0)) _camera))

(fn `UserConstructionScript`
  (bind _groundpath (`self.GroundPath`))
  (bind _showgroundpathdensityarrows (`self.ShowGroundPathDensityArrows`))
  (bind _camerapath (`self.CameraPath`))
  (bind _groundpath_2 (`self.GroundPath`))
  (bind _showgroundpathdensityarrows_2 (`self.ShowGroundPathDensityArrows`))
  (bind _grounddatapoints (`self.GroundDataPoints`))
  (bind _returnvalue (`SplineComponent.GetSplineLength` (`self.GroundPath`)))
  (bind _returnvalue_2 (- (`self.GroundPathPrecision`) 1))
  (bind _returnvalue_3 (- (`self.GroundPathPrecision`) 1))
  ;[1 1 1] Basic variable setups, stash the camera child as a simple variable for easier access later and place camera at 0 point of camera path
  (set `SplineComponent.Duration` (`self.CameraTrackDuration`) (`self.CameraPath`))
  (`SceneComponent.K2_SetWorldLocation` (`self.Camera`) (`SplineComponent.GetWorldLocationAtSplinePoint` (`self.CameraPath`) 0) false false)
  ;[1 1 1] Resize our camera track data array
  (if (`self.ClearCameraTrackData`)
    (`KismetArrayLibrary.Array_Clear` (`self.CameraDataPoints`))
    (set `self.ClearCameraTrackData` false))
  (`KismetArrayLibrary.Array_Resize` (`self.CameraDataPoints`) (`SplineComponent.GetNumberOfSplinePoints` (`self.CameraPath`)))
  ;[1 1 1] Calculate ground path to camera path ratio and durations for smooth translations between the two
  (set `self.CameraToPathRatio` (/ (`SplineComponent.GetSplineLength` (`self.CameraPath`)) (`SplineComponent.GetSplineLength` (`self.GroundPath`))))
  ;[1 1 1] Add arrows at camera splines to help visualize spline rotations
  (for _index (range (`SplineComponent.GetNumberOfSplinePoints` _camerapath))
    (if (`self.ShowCameraTrackArrows`)
      (bind (_output_fov _output_offset _output_rotation) (break `/Game/SplineCameraSystem/Struct_CameraTrackData` (`|GetArrayItem` (`self.CameraDataPoints`) _index)))
      (`AddComponent|NODE_AddArrowComponent-0` :`bManualAttachment` true :`RelativeTransform` (`KismetMathLibrary.MakeTransform` (+ (`SplineComponent.GetWorldLocationAtSplinePoint` _camerapath _index) _output_offset) _output_rotation)))
    (if (`self.ShowCameraTrackControlNumbers`)
      (bind _returnvalue_4 (`AddComponent|NODE_AddTextRenderComponent-0` :`bManualAttachment` true :`RelativeTransform` (`KismetMathLibrary.MakeTransform` (`KismetMathLibrary.MakeVector` (.x (`SplineComponent.GetWorldLocationAtSplinePoint` (`self.CameraPath`) _index)) (.y (`SplineComponent.GetWorldLocationAtSplinePoint` (`self.CameraPath`) _index)) (+ (.z (`SplineComponent.GetWorldLocationAtSplinePoint` (`self.CameraPath`) _index)) 20.0)))))
      (`TextRenderComponent.K2_SetText` _returnvalue_4 (`KismetTextLibrary.Conv_StringToText` (`KismetStringLibrary.Conv_IntToString` _index)))))
  ;[1 1 1] Setup path start and end trigger volumes
  (bind _returnvalue_5 (`AddComponent|NODE_AddBoxComponent-0` :`bManualAttachment` true :`RelativeTransform` (`KismetMathLibrary.MakeTransform` (`SplineComponent.GetWorldLocationAtSplinePoint` (`self.GroundPath`) 0))))
  (set `self.PathStartTrigger` _returnvalue_5)
  (`BoxComponent.SetBoxExtent` _returnvalue_5 (`self.StartEndTriggerExtents`) false)
  (bind _returnvalue_6 (`AddComponent|NODE_AddBoxComponent-1` :`bManualAttachment` true :`RelativeTransform` (`KismetMathLibrary.MakeTransform` (`SplineComponent.GetWorldLocationAtSplinePoint` _groundpath_2 (- (`SplineComponent.GetNumberOfSplinePoints` _groundpath_2) 1)))))
  (set `self.PathEndTrigger` _returnvalue_6)
  (`BoxComponent.SetBoxExtent` _returnvalue_6 (`self.StartEndTriggerExtents`) false)
  (bind _returnvalue_7 (`AddComponent|NODE_AddArrowComponent-2` :`bManualAttachment` true :`RelativeTransform` (`KismetMathLibrary.MakeTransform` (`SplineComponent.GetWorldLocationAtSplinePoint` (`self.GroundPath`) 0) (struct :`Pitch` 90.0) (2.0 2.0 2.0))))
  (set `self.PlayerPositionIndicator` _returnvalue_7)
  (`SceneComponent.SetVisibility` _returnvalue_7 _showgroundpathdensityarrows true)
  (`SceneComponent.SetHiddenInGame` _returnvalue_7 (not _showgroundpathdensityarrows) true)
  ;[1 1 1] Add some visualiztion arrows along the ground path to show density of checkpoints
  (for _index_2 (range (+ _returnvalue_2 1))
    (bind _returnvalue_8 (`AddComponent|NODE_AddArrowComponent-1` :`bManualAttachment` true :`RelativeTransform` (`KismetMathLibrary.MakeTransform` (`SplineComponent.GetWorldLocationAtDistanceAlongSpline` (`self.GroundPath`) (* (/ (`SplineComponent.GetSplineLength` (`self.GroundPath`)) (`KismetMathLibrary.Conv_IntToDouble` _returnvalue_2)) (`KismetMathLibrary.Conv_IntToDouble` _index_2))) (struct :`Pitch` 90.0))))
    (`SceneComponent.SetVisibility` _returnvalue_8 _showgroundpathdensityarrows_2 true)
    (`SceneComponent.SetHiddenInGame` _returnvalue_8 (not _showgroundpathdensityarrows_2) true))
  ;[1 1 1] Populate Ground Data Point Array
  (`KismetArrayLibrary.Array_Clear` _grounddatapoints)
  (`KismetArrayLibrary.Array_Resize` _grounddatapoints)
  (for _index_3 (range (+ _returnvalue_3 1))
    (bind _returnvalue_9 (* (`KismetMathLibrary.Conv_IntToDouble` _index_3) (/ _returnvalue (`KismetMathLibrary.Conv_IntToDouble` _returnvalue_3))))
    (bind _returnvalue_10 (`KismetMathLibrary.SelectFloat` (`KismetMathLibrary.SelectFloat` _returnvalue_9 (- _returnvalue 0.01) (< _returnvalue_9 _returnvalue)) 0.01 (> _returnvalue_9 0.0)))
    (`KismetArrayLibrary.Array_Add` (`self.GroundDataPoints`) (make `/Game/SplineCameraSystem/Struct_SplineLocation` (`SplineComponent.GetWorldLocationAtDistanceAlongSpline` _groundpath _returnvalue_10) (`SplineComponent.GetWorldRotationAtDistanceAlongSpline` _groundpath _returnvalue_10) _returnvalue_10))))